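; CardToTapManagerBP is a work-in-progress manager that converts mouse clicks into Tilemap grid coordinates, currently only printed for debugging.
; ClickButtonReleased deprojects the mouse position and calls Clicked, which repeats the deprojection instead of using the passed value.
; Clicked offsets that point by the tilemap's location and tile corner, then divides world X/Y by a hardcoded tile size and rounds.
; Alternative X/Z tile-index calculations remain disconnected.
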(fn `clickButtonReleased`
  (bind _returnvalue (`GameplayStatics.GetPlayerController` 0))
  (bind (_locationx _locationy) (`PlayerController.GetMousePosition` _returnvalue))
  (bind _worldposition (`GameplayStatics.DeprojectScreenToWorld` _returnvalue (`KismetMathLibrary.MakeVector2D` _locationx _locationy)))
  (`self.Clicked` _worldposition _worldposition))

(fn `Clicked`
  (params (WorldPos :type "Vector Structure") (WorldPos2 :type "Vector Structure"))
  (bind _returnvalue (`GameplayStatics.GetPlayerController` 0))
  (bind (_locationx _locationy) (`PlayerController.GetMousePosition` _returnvalue))
  (bind _rendercomponent (`PaperTileMapActor.RenderComponent` (`self.tilemap`)))
  (bind (_returnvalue_x _returnvalue_y) (`KismetMathLibrary.BreakVector` (- (`GameplayStatics.DeprojectScreenToWorld` _returnvalue (`KismetMathLibrary.MakeVector2D` _locationx _locationy)) (- (`SceneComponent.K2_GetComponentLocation` _rendercomponent) (`PaperTileMapComponent.GetTileCornerPosition` _rendercomponent 0 0 0 false)))))
  (`KismetSystemLibrary.PrintString` (`KismetStringLibrary.Conv_Vector2dToString` (`KismetMathLibrary.ToRounded2D` (/ (`KismetMathLibrary.MakeVector2D` _returnvalue_x _returnvalue_y) (16.0 16.0))))))

(fn `UserConstructionScript`)