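; Deck manager Blueprint that builds a shuffled card deck, deals it into hand slots and tracks the player's selected card.
; InitDeck expands DeckToBuild by copy count, draws the starting hand, then starts a delayed draw loop that continues while DeckWidget's UnusedBox has children and cards remain.
; Each draw moves the top card into Hand and a widget slot, hiding the deck when empty.
; Selection is single and toggleable, and the selected card can be rotated.
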(event `CheckDrawCards`
  (set `self.isDraw` true :!label _label)
  (`KismetSystemLibrary.Delay` (`self.TimerDrawCard`))
  (`self.DrawCard`)
  (if (and (> (`PanelWidget.GetChildrenCount` (`/Game/Widgets/DeckWidgetBP.UnusedBox` (`self.DeckWidget`))) 0) (> (`KismetArrayLibrary.Array_Length` (`self.deck`)) 0))
    (`self.CheckDrawCards`)
    (goto _label)
    (else
      (set `self.isDraw` false))))

(fn `cardSelected`
  (params (imgSelected :type "/Game/Widgets/CardHandBP Object Reference"))
  (bind _selectedcard (`self.selectedCard`))
  (for _array_element (`self.slotsHand`)
    (if (== _array_element imgSelected)
      (if (== _array_element _selectedcard)
        (`/Game/Widgets/CardHandBP.ChangeSelection` _selectedcard false)
        (set `self.selectedCard` null)
        (break)
        (else
          (if (`KismetSystemLibrary.IsValid` _selectedcard)
            (`/Game/Widgets/CardHandBP.ChangeSelection` _selectedcard false))
          (`/Game/Widgets/CardHandBP.ChangeSelection` _array_element true)
          (set `self.selectedCard` _array_element)
          (break))))))

(fn `DrawCard`
  (locals (card :type "/Game/Structs/Card Structure"))
  (bind _deck (`self.deck`))
  (bind _deck_2 (`self.deck`))
  (bind _output (`|GetArrayItem` _deck_2))
  (if (> (`KismetArrayLibrary.Array_Length` _deck_2) 0)
    (set `local.card` _output)
    (`KismetArrayLibrary.Array_Add` (`self.Hand`) _output)
    (`KismetArrayLibrary.Array_Remove` _deck)
    (if (== (`KismetArrayLibrary.Array_Length` _deck) 0)
      (set `Widget.Visibility` "Hidden" (`/Game/Widgets/DeckWidgetBP.Deck` (`self.DeckWidget`))))
    (bind _slothand (`/Game/Widgets/DeckWidgetBP.GetNewSlotHand` (`self.DeckWidget`)))
    (`KismetArrayLibrary.Array_Add` (`self.slotsHand`) _slothand)
    (`/Game/Widgets/CardHandBP.InitCard` _slothand (`local.card`))))

(fn `InitDeck`
  (for _array_element (`self.deckToBuild`)
    (for _ (range 1 (+ (`.nbToCreate_2_96B041D041F008449D80B9A0336EECC8` (break `/Game/Structs/Card` _array_element)) 1))
      (`KismetArrayLibrary.Array_Add` (`self.deck`) (`|Copy` _array_element))))
  (`KismetArrayLibrary.Array_Shuffle` (`self.deck`))
  (`self.InitDrawCards`))

(fn `InitDrawCards`
  (for _ (range (`self.nbCardToDrawOnStart`))
    (`self.DrawCard`))
  (`self.CheckDrawCards`))

(fn `RotateSelection`
  (bind _selectedcard (`self.selectedCard`))
  (`/Engine/EditorBlueprintResources/StandardMacros.IsValid` _selectedcard
    (:`Is Valid`
      (`/Game/Widgets/CardHandBP.AddRotation` _selectedcard))))

(fn `setCardManagerInWidget`
  (`/Game/Widgets/DeckWidgetBP.SetDeckManager` (`self.DeckWidget`) self))

(fn `UserConstructionScript`)