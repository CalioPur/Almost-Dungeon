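; SpawnGridBP builds the bordered tile-map play grid at BeginPlay and starts the card deck.
; It recreates the Paper2D tile map at the configured size plus a one-tile margin, drawing horizontal and vertical contour walls around an interior filled with holes.
; A Start tile lands on a random row of the first interior column.
; It then creates the deck widget, hands it to DeckManager and calls InitDeck.
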(event `self.ReceiveBeginPlay`
  (bind _deckmanager (`self.DeckManager`))
  (`self.ResetTileMap`)
  (`self.SpawnWalls`)
  (`self.SpawnHole`)
  (`PaperTileMapComponent.SetTile` (`PaperTileMapActor.RenderComponent` (`self.TileMap`)) 1 (`KismetMathLibrary.RandomIntegerInRange` 1 (`self.SizeY`)) 0 (`self.Start`))
  (bind _returnvalue (`|CreateWidget` "/Game/Widgets/DeckWidgetBP.DeckWidgetBP_C"))
  (bind _output_get (set `self.WidgetDeck` _returnvalue))
  (`UserWidget.AddToViewport` _output_get 0)
  (set `/Game/Blueprints/DeckManagerBP.DeckWidget` (`self.WidgetDeck`) _deckmanager)
  (`/Game/Blueprints/DeckManagerBP.InitDeck` _deckmanager))

(fn `ResetTileMap`
  (`PaperTileMapComponent.CreateNewTileMap` (`PaperTileMapActor.RenderComponent` (`self.TileMap`)) (+ (`self.SizeX`) 2) (+ (`self.SizeY`) 2) 16 16 1.0 true))

(fn `SpawnHole`
  (for _index (range 1 (+ (`self.SizeY`) 1))
    (for _index_2 (range 1 (+ (`self.SizeX`) 1))
      (`PaperTileMapComponent.SetTile` (`PaperTileMapActor.RenderComponent` (`self.TileMap`)) _index_2 _index 0 (`self.Hole`)))))

(fn `SpawnWalls`
  (bind _contourmapvertical (`self.ContourMapVertical`))
  (bind _contourmaphorizontal (`self.ContourMapHorizontal`))
  (bind _rendercomponent (`PaperTileMapActor.RenderComponent` (`self.TileMap`)))
  (for _index (range (+ (+ (`self.SizeX`) 1) 1))
    (`PaperTileMapComponent.SetTile` _rendercomponent _index 0 0 _contourmaphorizontal)
    (`PaperTileMapComponent.SetTile` _rendercomponent _index (+ (`self.SizeY`) 1) 0 _contourmaphorizontal))
  (for _index_2 (range (+ (+ (`self.SizeY`) 1) 1))
    (`PaperTileMapComponent.SetTile` _rendercomponent 0 _index_2 0 _contourmapvertical)
    (`PaperTileMapComponent.SetTile` _rendercomponent (+ (`self.SizeX`) 1) _index_2 0 _contourmapvertical)))

(fn `UserConstructionScript`)